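; Pickup Blueprint for an item that the player collects by pressing the Pick input while inside its trigger.
; Trigger overlap with MyFPCharacter toggles IsPickupable and shows or removes a PickupPrompt widget.
; On Pick, it passes ItemType to AddItemCount on MyGameMode_BP, found through GetActorOfClass.
; PlayPickupEffect then plays a water-drop sound and RadialBurst effect at its location and destroys the actor.
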(event `InputAction|Pick` :consume false
  (params (Key :type "Key Structure"))
  (:`Pressed`
    (if (`self.IsPickupable`)
      (bind _returnvalue (`GameplayStatics.GetActorOfClass` "/Game/Blueprints/MyGameMode_BP.MyGameMode_BP_C"))
      (`/Game/Blueprints/MyGameMode_BP.AddItemCount` _returnvalue (`self.ItemType`))
      (`self.Play Pickup Effect`))))

(event `Play Pickup Effect`
  (`GameplayStatics.SpawnSoundAtLocation` "/Game/Audio/single_water_drop.single_water_drop" (`self.K2_GetActorLocation`) (struct) 1.0 1.0 0.3 null null)
  (`NiagaraFunctionLibrary.SpawnSystemAtLocation` "/Niagara/DefaultAssets/Templates/Systems/RadialBurst.RadialBurst" (`self.K2_GetActorLocation`) (struct) (0.5 0.5 0.5))
  (`self.K2_DestroyActor`))

(event `self.Trigger.OnComponentBeginOverlap`
  (params (OverlappedComponent :type "PrimitiveComponent Object Reference") (OtherActor :type "Actor Object Reference") (OtherComp :type "PrimitiveComponent Object Reference") (OtherBodyIndex :type Integer) (bFromSweep :type Boolean) (SweepResult :type "HitResult Structure (by ref)"))
  (cast `/Game/Blueprints/MyFPCharacter` OtherActor)
  (set `self.IsPickupable` true)
  (bind _returnvalue (`|CreateWidget` "/Game/Blueprints/HUD/PickupPrompt.PickupPrompt_C"))
  (`UserWidget.AddToViewport` _returnvalue 0))

(event `self.Trigger.OnComponentEndOverlap`
  (params (OverlappedComponent :type "PrimitiveComponent Object Reference") (OtherActor :type "Actor Object Reference") (OtherComp :type "PrimitiveComponent Object Reference") (OtherBodyIndex :type Integer))
  (cast `/Game/Blueprints/MyFPCharacter` OtherActor)
  (set `self.IsPickupable` false)
  (`Widget.RemoveFromParent` (stale `self.Trigger.OnComponentBeginOverlap` _returnvalue)))

(fn `UserConstructionScript`)