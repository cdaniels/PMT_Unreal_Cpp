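; Game mode that runs timed rounds of an item-collection game, tallying fire, extinguisher and life potion pickups.
; Tick uses a one-second Delay as a countdown; at zero it computes player and team scores, shows RoundOver and pauses with the cursor visible.
; NextRound advances the round, resets the timer and rebuilds the item, timer and round HUD.
; Helpers reset player counts, compute a robot-based team score and open an end-of-round survey.
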(event `self.ReceiveBeginPlay`
  (`self.CreateHUD`))

(event `self.ReceiveTick`
  (params (DeltaSeconds :type "Float (single-precision)"))
  ;[1 1 1] Decrement Time untill clock runs out
  (`KismetSystemLibrary.Delay` 1.0)
  (if (== (`self.Seconds`) 0)
    (if (== (`self.Minutes`) 0)
      ;[1 1 1] Handle End of Round
      (`self.UpdatePlayerScore`)
      (`self.UpdateTeamScore_ForPlayer`)
      (bind _returnvalue (`|CreateWidget` "/Game/Blueprints/Menus/RoundOver.RoundOver_C"))
      (`UserWidget.AddToViewport` _returnvalue 0)
      ;[1 1 1] Enter Menu Mode
      (set `PlayerController.bShowMouseCursor` true (`GameplayStatics.GetPlayerController` 0))
      (`GameplayStatics.SetGamePaused` true)
      (else
        (set `self.Seconds` 59)
        (set `self.Minutes` (- (`self.Minutes`) 1))))
    (else
      (set `self.Seconds` (- (`self.Seconds`) 1)))))

(fn `AddItemCount`
  (params (ItemType :type "/Game/Blueprints/Pickups/PickupableItems Enum" :default "NewEnumerator0"))
  (switch `/Game/Blueprints/Pickups/PickupableItems` ItemType
    (:`NewEnumerator0`
      (set `self.Player_ExtinguisherCount_Int` (+ (`self.Player_ExtinguisherCount_Int`) 1)))
    (:`NewEnumerator1`
      (set `self.Player_FireCount_Int` (+ (`self.Player_FireCount_Int`) 1)))
    (:`NewEnumerator2`
      (set `self.Player_LifePotionCount_Int` (+ (`self.Player_LifePotionCount_Int`) 1)))))

(fn `CreateHUD`
  (bind _returnvalue (`|CreateWidget` "/Game/Blueprints/HUD/ItemCount.ItemCount_C"))
  (`UserWidget.AddToViewport` _returnvalue 0)
  (bind _returnvalue_2 (`|CreateWidget` "/Game/Blueprints/HUD/Timer.Timer_C"))
  (`UserWidget.AddToViewport` _returnvalue_2 0)
  (bind _returnvalue_3 (`|CreateWidget` "/Game/Blueprints/HUD/RoundNumber.RoundNumber_C"))
  (`UserWidget.AddToViewport` _returnvalue_3 0))

(fn `NextRound`
  ;[1 1 1] Increment Round Number
  (set `self.Round_Number` (+ (`self.Round_Number`) 1))
  ;[1 1 1] Reset Timer
  (set `self.Minutes` 1)
  (set `self.Seconds` 0)
  ;[1 1 1] Exit menu mode
  (`WidgetLayoutLibrary.RemoveAllWidgets`)
  (set `PlayerController.bShowMouseCursor` false (`GameplayStatics.GetPlayerController` 0))
  (`GameplayStatics.SetGamePaused` false)
  (`self.CreateHUD`))

(fn `OpenEndOfRoundSurvey`
  (`WidgetLayoutLibrary.RemoveAllWidgets`)
  (bind _returnvalue (`|CreateWidget` "/Game/Blueprints/Menus/EndOfRoundSurvey.EndOfRoundSurvey_C"))
  (`UserWidget.AddToViewport` _returnvalue 0))

(fn `ResetPlayerItemCount`
  (set `self.Player_FireCount_Int` 0)
  (set `self.Player_ExtinguisherCount_Int` 0)
  (set `self.Player_LifePotionCount_Int` 0))

(fn `UpdatePlayerScore`
  (set `self.Player_Score_Int` (* (`self.Player_LifePotionCount_Int`) 100)))

(fn `UpdateTeamScore_ForPlayer`
  (set `self.Team_Score_Int` (- (* (`self.Player_ExtinguisherCount_Int`) 100) (+ (* (`self.Player_FireCount_Int`) 100) (* (`self.Player_LifePotionCount_Int`) 100)))))

(fn `UpdateTeamScore_ForRobot`
  (set `self.Team_Score_Int` (- (* (`self.Robot_ExtinguisherCount_Int`) 100) (+ (* (`self.Robot_FireCount_Int`) 100) (* (`self.Robot_LifePotionCount_Int`) 100)))))

(fn `UserConstructionScript`)