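; Actor component that scatters weighted random actors across the tiles of its owning RoomGenerator when play begins.
; It gathers floor tiles, adding corridors unless RoomOnly is set, then draws tiles from the generator's random stream until Quantity is reached.
; Tiles that fail a spacing check against the last spawn are rerolled.
; SpawnList entries are rolled in order, and the first success spawns there and removes that tile.
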(event `self.ReceiveBeginPlay`
  (`self.TriggerSpawnThings`))

(event `TriggerSpawnThings`
  (bind _asroom_generator (cast `/Game/Blueprints/ProceduralRooms/RoomGenerator` (`self.GetOwner`)))
  (bind _output_get (set `self.Environment` _asroom_generator))
  (if (`self.RoomOnly?`)
    (bind _floortiles (`/Game/Blueprints/ProceduralRooms/RoomGenerator.FloorTiles` _output_get))
    (set `self.SpawnableTiles` _floortiles)
    (else
      (set `self.SpawnableTiles` _floortiles)
      (`KismetArrayLibrary.Array_Append` (`self.SpawnableTiles`) (`/Game/Blueprints/ProceduralRooms/RoomGenerator.CorridorTiles` _output_get))))
  (`self.SpawnItems`))

(fn `SpawnItems`
  (locals (ItemsSpawned :type Integer) (TileIndex :type Integer :default 0) (LastLocation :type "Vector Structure" :default (0.0 0.0 0.0)))
  (bind _spawnlist (`self.SpawnList`))
  (bind _returnvalue (`KismetMathLibrary.Conv_IntVectorToVector` (`|GetArrayItem` (`self.SpawnableTiles`) (`local.TileIndex`))))
  ;[1 1 1] While spawns are less than desired quantity
  (while (> (`self.Quantity`) (`local.ItemsSpawned`))
    ;[1 1 1] Get random tile, test if minimum distance is respected
    (bind _output_get (set `local.TileIndex` (`KismetMathLibrary.RandomIntegerInRangeFromStream` 0 (`KismetArrayLibrary.Array_LastIndex` (`self.SpawnableTiles`)) (`/Game/Blueprints/ProceduralRooms/RoomGenerator.Stream` (`self.Environment`))) :!label _label))
    (if (== (* (`KismetMathLibrary.Conv_IntVectorToVector` (`|GetArrayItem` (`self.SpawnableTiles`) _output_get)) (`/Game/Blueprints/ProceduralRooms/RoomGenerator.Scale` (`self.Environment`))) (`local.LastLocation`) :`ErrorTolerance` (`self.MinDistance`))
      (goto _label)
      (else
        ;[1 1 1] Loop through spawn list, and find a next item to spawn given spawn chances
        (bind _keys (`BlueprintMapLibrary.Map_Keys` _spawnlist))
        (for _array_element _keys
          (if (`KismetMathLibrary.RandomBoolWithWeightFromStream` (`BlueprintMapLibrary.Map_Find` _spawnlist _array_element) (`/Game/Blueprints/ProceduralRooms/RoomGenerator.Stream` (`self.Environment`)))
            (`|ExecutionSequence`
              (:`then_0`
                ;[1 1 1] Spawn actor, remove item from list, and increment itemsSpawned
                (`|SpawnActorFromClass` _array_element (`KismetMathLibrary.Conv_VectorToTransform` (+ (+ (* _returnvalue (`/Game/Blueprints/ProceduralRooms/RoomGenerator.Scale` (`self.Environment`))) (`Actor.K2_GetActorLocation` (`self.GetOwner`))) (`self.Offset`))) "Undefined" "OverrideRootScale" null null)
                (set `local.LastLocation` _returnvalue)
                (`KismetArrayLibrary.Array_Remove` (`self.SpawnableTiles`) (`local.TileIndex`)) ; remove tile from list so no ne item can be spaned there
                (`/Engine/EditorBlueprintResources/StandardMacros.IncrementInt` (`local.ItemsSpawned`)))
              (:`then_1`
                (break)))))))))