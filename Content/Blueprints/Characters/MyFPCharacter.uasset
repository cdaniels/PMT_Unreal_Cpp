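; First-person player character Blueprint that handles movement and look input and can save the player's score.
; Movement axes push the character along forward and right vectors built from control-rotation yaw only, so pitch does not affect direction.
; Look axes feed controller pitch and yaw, clamped to a unit range.
; SaveScore creates a fresh MySaveGame object, stores the given score and writes it to the "ScoreSlot" save slot.
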(event `InputAxis|Forwards/Backward`
  (params (AxisValue :type "Float (single-precision)"))
  (`self.AddMovementInput` (`KismetMathLibrary.GetForwardVector` (`KismetMathLibrary.MakeRotator` 0.0 0.0 (.yaw (`self.GetControlRotation`)))) AxisValue))

(event `InputAxis|Left/Right`
  (params (AxisValue :type "Float (single-precision)"))
  (`self.AddMovementInput` (`KismetMathLibrary.GetRightVector` (`KismetMathLibrary.MakeRotator` 0.0 0.0 (.yaw (`self.GetControlRotation`)))) AxisValue))

(event `InputAxis|LookUp/LookDown`
  (params (AxisValue :type "Float (single-precision)"))
  (`self.AddControllerPitchInput` (`KismetMathLibrary.FClamp` AxisValue -1.0)))

(event `InputAxis|LookLeft/LookRight`
  (params (AxisValue :type "Float (single-precision)"))
  (`self.AddControllerYawInput` (`KismetMathLibrary.FClamp` AxisValue -1.0)))

(fn `SaveScore`
  (params (PlayerScore :type Integer))
  (bind _returnvalue (`GameplayStatics.CreateSaveGameObject` "/Game/Blueprints/MySaveGame.MySaveGame_C"))
  (bind _output_get (set `self.SaveGameRef` _returnvalue))
  (set `/Game/Blueprints/MySaveGame.PlayerScore` PlayerScore _output_get)
  (`GameplayStatics.SaveGameToSlot` _output_get "ScoreSlot"))

(fn `UserConstructionScript`)