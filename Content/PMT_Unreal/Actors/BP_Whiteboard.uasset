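; BP_Whiteboard is a whiteboard actor that draws marker spots onto a render target.
; On BeginPlay it creates a dynamic instance of M_Whiteboard_Marker and clears RT_Whiteboard to black.
; Its DrawonWhiteboard event takes a 2D location, sets it and a fixed brush size on that instance, then draws the material to the render target and prints the location as debug output.
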(event `self.ReceiveBeginPlay`
  (bind _returnvalue (`KismetMaterialLibrary.CreateDynamicMaterialInstance` "/Game/PMT_Unreal/Materials/M_Whiteboard_Marker.M_Whiteboard_Marker"))
  (set `self.WhiteboardMarker_MI` _returnvalue)
  (`KismetRenderingLibrary.ClearRenderTarget2D` "/Game/PMT_Unreal/Materials/RT_Whiteboard.RT_Whiteboard"))

(event `Draw on Whiteboard`
  (params (LocationToDraw :type "Vector2D Structure"))
  (bind _whiteboardmarker_mi (`self.WhiteboardMarker_MI`))
  (bind _returnvalue (`KismetMathLibrary.Conv_VectorToLinearColor` (`KismetMathLibrary.Conv_Vector2DToVector` LocationToDraw)))
  (`MaterialInstanceDynamic.SetVectorParameterValue` _whiteboardmarker_mi "DrawLocation" _returnvalue)
  (`MaterialInstanceDynamic.SetScalarParameterValue` _whiteboardmarker_mi "DrawSize" 0.03)
  (`KismetRenderingLibrary.DrawMaterialToRenderTarget` "/Game/PMT_Unreal/Materials/RT_Whiteboard.RT_Whiteboard" _whiteboardmarker_mi)
  (`KismetSystemLibrary.PrintString` (`KismetStringLibrary.Conv_ColorToString` _returnvalue)))

(fn `UserConstructionScript`)