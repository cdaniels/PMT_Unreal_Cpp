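; World map component that shows the player's position on a toggleable UI map, switching mouse cursor and input mode with visibility.
; TargetPoints named UpperLeft and LowerRight define the world bounds, used to convert between world locations and map positions.
; InitializeMap sets up the W_Main widget hidden, and OnPlayerMoved repositions the centered player icon.
; When masking is enabled, the player's map position becomes a UV that marks areas searched, like fog of war.
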(event `self.ReceiveBeginPlay`)

(event `InitializeMap`
  (params (Player :type "Character Object Reference"))
  (bind _mapreference (`self.MapReference`))
  (bind _mapreference_2 (`self.MapReference`))
  (`self.InitializeMapPopup`)
  (if (`self.AreCornersValid?`)
    ;[1 1 1] Construct widget and add to Viewport
    (`/Engine/EditorBlueprintResources/StandardMacros.IsValid` Player
      (:`Is Valid`
        (set `self.Player` Player)
        (`/Game/PMT_Unreal/Widgets/W_WorldMap.Initialize` (`self.MapReference`) self)
        (set `self.OriginalPlayerSize` (`KismetMathLibrary.MakeVector2D` (`KismetMathLibrary.Conv_IntToDouble` (`/Game/PMT_Unreal/Widgets/W_WorldMap.PlayerSizeX` _mapreference)) (`KismetMathLibrary.Conv_IntToDouble` (`/Game/PMT_Unreal/Widgets/W_WorldMap.PlayerSizeY` _mapreference))))
        (set `self.OriginalMapSize` (`KismetMathLibrary.MakeVector2D` (`KismetMathLibrary.Conv_IntToDouble` (`/Game/PMT_Unreal/Widgets/W_WorldMap.MapSizeX` _mapreference_2)) (`KismetMathLibrary.Conv_IntToDouble` (`/Game/PMT_Unreal/Widgets/W_WorldMap.MapSizeY` _mapreference_2))))
        (`self.ShowMap` false)
        (`UserWidget.AddToViewport` (`self.MainReference`) 0))
      (:`Is Not Valid`
        (`KismetSystemLibrary.PrintString` "Error: Player is not valid in BPC_WorldMap")))))

(event `OnPlayerMoved`
  (`self.UpdatePlayerPositionOnMap`))

(fn `AreCornersValid?`
  (returns (ReturnValue :type Boolean))
  (return (and (`KismetSystemLibrary.IsValid` (`self.UpperLeftCorner`)) (`KismetSystemLibrary.IsValid` (`self.LowerRightCorner`)))))

(fn `CenterIconPosition`
  (params (Location :type "Vector2D Structure") (WidgetSize :type "Vector2D Structure"))
  (returns (CenteredPosition :type "Vector2D Structure"))
  (bind (_x _y) (`KismetMathLibrary.BreakVector2D` Location))
  (bind (_x_2 _y_2) (`KismetMathLibrary.BreakVector2D` (`local.WidgetSize`)))
  (return (`KismetMathLibrary.MakeVector2D` (- _x (/ _x_2 2.0)) (- _y (/ _y_2 2.0)))))

(fn `GetMapHeight`
  (returns (Out :type "Float (double-precision)"))
  (bind (_returnvalue_x _returnvalue_y) (`KismetMathLibrary.BreakVector` (`Actor.K2_GetActorLocation` (`self.LowerRightCorner`))))
  (bind (_returnvalue_x_2 _returnvalue_y_2) (`KismetMathLibrary.BreakVector` (`Actor.K2_GetActorLocation` (`self.UpperLeftCorner`))))
  (return (select `bool` (`self.AreCornersValid?`) :`true` (`KismetMathLibrary.Abs` (- _returnvalue_y _returnvalue_y_2)))))

(fn `GetMapWidth`
  (returns (Out :type "Float (double-precision)"))
  (bind _returnvalue_x (`KismetMathLibrary.BreakVector` (`Actor.K2_GetActorLocation` (`self.LowerRightCorner`))))
  (bind _returnvalue_x_2 (`KismetMathLibrary.BreakVector` (`Actor.K2_GetActorLocation` (`self.UpperLeftCorner`))))
  (return (select `bool` (`self.AreCornersValid?`) :`true` (`KismetMathLibrary.Abs` (- _returnvalue_x _returnvalue_x_2)))))

(fn `GetWidgetSize`
  (params (Widget :type "Widget Object Reference"))
  (returns (Size :type "Vector2D Structure"))
  (bind (_x _y) (`KismetMathLibrary.BreakVector2D` (`Widget.GetDesiredSize` Widget)))
  (bind (_x_2 _y_2) (`KismetMathLibrary.BreakVector2D` (`WidgetLayoutLibrary.GetViewportSize`)))
  (return (`KismetMathLibrary.MakeVector2D` (* _x (/ _x_2 1920.0)) (* _y (/ _y_2 1080.0)))))

(fn `InitializeMapPopup`
  (`self.InitializeMapCorners`
    (:`Completed`
      (if true
        (bind _returnvalue (`|CreateWidget` "/Game/PMT_Unreal/Widgets/W_Main.W_Main_C"))
        (bind _output_get (set `self.MainReference` _returnvalue))
        (set `self.MapReference` (`/Game/PMT_Unreal/Widgets/W_Main.WorldMap` _output_get))
        (`/Game/PMT_Unreal/Widgets/W_UnsearchedAreaMask.Reset Searched Area` (`/Game/PMT_Unreal/Widgets/W_WorldMap.UnsearchedMask` (`self.MapReference`)))
        (`self.ShowMap` true)))))

(fn `MapAreaLocationToMapPosition`
  (params (Location :type "Vector Structure"))
  (returns (Out :type "Vector2D Structure"))
  (bind _mapreference (`self.MapReference`))
  (bind (_x _y) (`KismetMathLibrary.BreakVector2D` (`self.RelativeLocationInMapArea` Location)))
  (return (`KismetMathLibrary.MakeVector2D` (- (`KismetMathLibrary.Conv_IntToDouble` (`/Game/PMT_Unreal/Widgets/W_WorldMap.MapSizeX` _mapreference)) (* (/ _x (`self.GetMapWidth`)) (`KismetMathLibrary.Conv_IntToDouble` (`/Game/PMT_Unreal/Widgets/W_WorldMap.MapSizeX` _mapreference)))) (- (`KismetMathLibrary.Conv_IntToDouble` (`/Game/PMT_Unreal/Widgets/W_WorldMap.MapSizeY` _mapreference)) (* (`KismetMathLibrary.Conv_IntToDouble` (`/Game/PMT_Unreal/Widgets/W_WorldMap.MapSizeY` _mapreference)) (/ _y (`self.GetMapHeight`)))))))

(fn `MapPositionToUV`
  (params (Position :type "Vector2D Structure"))
  (returns (Coordinates :type "Vector2D Structure"))
  (bind (_x _y) (`KismetMathLibrary.BreakVector2D` Position))
  (bind _mapreference (`self.MapReference`))
  (return (`KismetMathLibrary.MakeVector2D` (/ _x (`KismetMathLibrary.Conv_IntToDouble` (`/Game/PMT_Unreal/Widgets/W_WorldMap.MapSizeX` _mapreference))) (/ _y (`KismetMathLibrary.Conv_IntToDouble` (`/Game/PMT_Unreal/Widgets/W_WorldMap.MapSizeY` _mapreference))))))

(fn `MapPositionToWorldLocation`
  (params (Position :type "Vector2D Structure"))
  (returns (Location :type "Vector Structure"))
  (locals (LocalPercentageInX :type "Float (double-precision)" :default 0.0) (LocalPercentageInY :type "Float (double-precision)" :default 0.0))
  (bind (_x _y) (`KismetMathLibrary.BreakVector2D` Position))
  (bind _mapreference (`self.MapReference`))
  (set `local.LocalPercentageInX` (/ _x (`KismetMathLibrary.Conv_IntToDouble` (`/Game/PMT_Unreal/Widgets/W_WorldMap.MapSizeX` _mapreference))))
  (set `local.LocalPercentageInY` (/ _y (`KismetMathLibrary.Conv_IntToDouble` (`/Game/PMT_Unreal/Widgets/W_WorldMap.MapSizeY` _mapreference))))
  (return (`KismetMathLibrary.MakeVector` (- (.x (`Actor.K2_GetActorLocation` (`self.UpperLeftCorner`))) (* (`self.GetMapHeight`) (`local.LocalPercentageInY`))) (+ (.y (`Actor.K2_GetActorLocation` (`self.UpperLeftCorner`))) (* (`self.GetMapWidth`) (`local.LocalPercentageInX`))))))

(fn `RelativeLocationInMapArea`
  (params (WorldLocation :type "Vector Structure"))
  (returns (MapLocation :type "Vector2D Structure"))
  (bind (_returnvalue_x _returnvalue_y) (`KismetMathLibrary.BreakVector` (`Actor.K2_GetActorLocation` (`self.UpperLeftCorner`))))
  (return (`KismetMathLibrary.MakeVector2D` (`KismetMathLibrary.Abs` (- (.x WorldLocation) _returnvalue_x)) (`KismetMathLibrary.Abs` (- (.y WorldLocation) _returnvalue_y)))))

(fn `ShowMap`
  (params (`Show?` :type Boolean))
  (bind _returnvalue (`GameplayStatics.GetPlayerController` 0))
  (bind _mapreference (`self.MapReference`))
  (if (!= `Show?` (`self.Visible?`))
    (bind _output_get (set `self.Visible?` `Show?`))
    (if _output_get
      (`Widget.SetVisibility` _mapreference "SelfHitTestInvisible")
      (`Widget.SetVisibility` (`self.MainReference`) "SelfHitTestInvisible")
      (set `PlayerController.bShowMouseCursor` true _returnvalue)
      (`WidgetBlueprintLibrary.SetInputMode_GameAndUIEx` _returnvalue _mapreference)
      (`self.UpdatePlayerPositionOnMap`)
      (return)
      (else
        (`Widget.SetVisibility` _mapreference "Hidden")
        (`Widget.SetVisibility` (`self.MainReference`) "Hidden")
        (set `PlayerController.bShowMouseCursor` false _returnvalue)
        (`WidgetBlueprintLibrary.SetInputMode_GameOnly` _returnvalue)
        (return)))
    (else
      (return))))

(fn `ToggleVisibility`
  (`self.ShowMap` (not (`self.Visible?`)))
  (return))

(fn `UpdatePlayerPositionOnMap`
  (bind _mapreference (`self.MapReference`))
  (bind _out (`self.MapAreaLocationToMapPosition` (`Actor.K2_GetActorLocation` (`self.Player`))))
  (`Widget.SetRenderTranslation` (`/Game/PMT_Unreal/Widgets/W_WorldMap.PlayerBox` (`self.MapReference`)) (`self.CenterIconPosition` _out (`self.OriginalPlayerSize`)))
  (if (`/Game/PMT_Unreal/Widgets/W_WorldMap.MaskUnsearchedArea?` _mapreference)
    (`/Game/PMT_Unreal/Widgets/W_WorldMap.MarkAreaSearched` _mapreference (`self.MapPositionToUV` _out))
    (return)
    (else
      (return))))